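; MainCharacter_BP is the Warrior main character Blueprint, adding debug-style key bindings and a level restart when the character is destroyed.
; The C, R and T keys call functions defined outside this graph to show pickup locations, save the game and load the game.
; The Destroyed event reopens the current level by name.
; A health-based restart check and a quit call are left unwired, and Tick is empty.
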(event `Key|C`
  (params (Key :type "Key Structure"))
  (:`Pressed`
    (`self.ShowPickupLocations`)))

(event `Key|R`
  (params (Key :type "Key Structure"))
  (:`Pressed`
    (`self.SaveGame`)))

(event `Key|T`
  (params (Key :type "Key Structure"))
  (:`Pressed`
    (`self.LoadGame` true)))

(event `self.ReceiveDestroyed`
  (bind _returnvalue (`GameplayStatics.GetCurrentLevelName` true))
  (`GameplayStatics.OpenLevel` (`KismetStringLibrary.Conv_StringToName` _returnvalue)))

(event `self.ReceiveTick`
  (params (DeltaSeconds :type "Float (single-precision)")))

(fn `UserConstructionScript`)